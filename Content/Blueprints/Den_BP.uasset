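; Den_BP is a numbered den actor that spawns AI characters.
; The construction script shows DenNumber on the Number text.
; SpawnAPawn creates an AIController_BP with FinishingPoint as its destination and DenNumber as pawn type, then spawns an AIChar in DenColor at the den, plays a wolf roar and has the controller possess it.
; The event graph is empty, so spawning relies on an external call.
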(fn `SpawnAPawn`
  (`|ExecutionSequence`
    (:`then_0`
      (bind _returnvalue (`|SpawnActorFromClass` "/Game/Blueprints/AIController_BP.AIController_BP_C" (`KismetMathLibrary.MakeTransform` (0.0 0.0 0.0)) "Undefined" "OverrideRootScale" null (`self.FinishingPoint`) (`self.DenNumber`) null)))
    (:`then_1`
      (bind _returnvalue_2 (`|SpawnActorFromClass` "/Game/Blueprints/AIChar.AIChar_C" (`KismetMathLibrary.MakeTransform` (.location (`self.GetTransform`)) (.rotation (`self.GetTransform`))) "Undefined" "OverrideRootScale" null (`self.DenColor`) null))
      (`GameplayStatics.PlaySoundAtLocation` "/Game/SoundEffects/WolfRoar.WolfRoar" (`self.K2_GetActorLocation` _returnvalue_2) (struct) 1.0 1.0 0.0 null null null)
      (`Controller.Possess` _returnvalue _returnvalue_2))))

(fn `UserConstructionScript`
  (`TextRenderComponent.K2_SetText` (`self.Number`) (`KismetTextLibrary.Conv_IntToText` (`self.DenNumber`))))