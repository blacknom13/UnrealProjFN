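; AI-controlled wolf character that handles its own Niagara and sound effects for arriving, evaporating and traveling through a portal.
; The construction script snaps eye and paw-dust effects to mesh sockets and tints the eyes.
; Events stop dust on arrival, evaporate the wolf, feed the assigned portal's location into a pull effect, or spawn a flash.
; Effect-finished callbacks and the flash notify the AI controller when each sequence ends.
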(event `AssignPortal`
  (params (PortalRef :type "/Game/Blueprints/Portal Object Reference"))
  (set `self.PortalRef` PortalRef))

(event `/Game/Blueprints/General_BPI.DestinationReached`
  (params (AIChar :type "/Game/Blueprints/AIChar Object Reference"))
  (for _array_element (`|MakeArray` (`self.DustRightHand`) (`self.DustLeftHand`) (`self.DustRightLeg`) (`self.DustLeftLeg`))
    (`ActorComponent.SetActive` _array_element false false)
    (`GameplayStatics.PlaySoundAtLocation` "/Game/SoundEffects/Wolf.Wolf" (`self.K2_GetActorLocation`) (struct) 1.0 1.0 0.0 null null null)
    (set `self.ReachedEndPoint` true)))

(event `SpawnEvaporation`
  (`ActorComponent.SetActive` (`self.Evaporation`) true false)
  (`KismetSystemLibrary.Delay` 2.0)
  (`GameplayStatics.PlaySoundAtLocation` "/Game/SoundEffects/Evaporating_Cue.Evaporating_Cue" (`self.K2_GetActorLocation`) (struct) 1.0 1.0 0.0 null null null)
  (`SceneComponent.SetVisibility` (`self.Mesh`) false true))

(event `PortWolf`
  (`self.EvaporatePortal`)
  (`KismetSystemLibrary.Delay` 2.0)
  (`GameplayStatics.PlaySoundAtLocation` "/Game/SoundEffects/PortalSound.PortalSound" (`self.K2_GetActorLocation`) (struct) 1.0 1.0 0.0 null null null)
  (`SceneComponent.SetVisibility` (`self.Mesh`) false true))

(event `SpawnPortingFlash`
  (`ActorComponent.SetActive` (`self.FX_PortalWolf`) false false)
  (`NiagaraFunctionLibrary.SpawnSystemAtLocation` "/Game/NiagaraEffects/FX_PortalFlash.FX_PortalFlash" (`self.K2_GetActorLocation`))
  (`KismetSystemLibrary.Delay` 0.2)
  (message `/Game/Blueprints/General_BPI.EndInteract` (`AIBlueprintHelperLibrary.GetAIController` self)))

(event `EvaporatePortal`
  (bind _evapportal (`self.EvapPortal`))
  (`ActorComponent.SetActive` _evapportal true false)
  (`NiagaraComponent.SetVariableVec3` _evapportal "User.PortalLocation" (`self.K2_GetActorLocation` (`self.PortalRef`)))
  (`NiagaraComponent.SetVariableVec3` _evapportal "User.PullToCenter" (0.0 0.0 0.0)))

(event `self.Evaporation.OnSystemFinished`
  (params (PSystem :type "NiagaraComponent Object Reference"))
  (bind _asaicontroller_bp (cast `/Game/Blueprints/AIController_BP` (`self.GetController`)))
  (`/Game/Blueprints/AIController_BP.EvaporateFinished` _asaicontroller_bp))

(event `self.EvapPortal.OnSystemFinished`
  (params (PSystem :type "NiagaraComponent Object Reference"))
  (bind _asaicontroller_bp (cast `/Game/Blueprints/AIController_BP` (`self.GetController`)))
  (`/Game/Blueprints/General_BPI.EndInteract` _asaicontroller_bp))

(fn `UserConstructionScript`
  (bind _lefteye (`self.LeftEye`))
  (bind _color (`self.Color`))
  (bind _color_2 (`self.Color`))
  (bind _righteye (`self.RightEye`))
  (`SceneComponent.K2_AttachToComponent` (`self.RightEye`) (`self.Mesh`) "RightEye" "SnapToTarget" "SnapToTarget" "SnapToTarget" false)
  (`SceneComponent.K2_AttachToComponent` (`self.LeftEye`) (`self.Mesh`) "LeftEye" "SnapToTarget" "SnapToTarget" "SnapToTarget" false)
  (`NiagaraComponent.SetVariableLinearColor` _lefteye "EyesColor" _color)
  (`NiagaraComponent.SetVariableLinearColor` _lefteye "SparksColor" (* _color (`KismetMathLibrary.MakeColor` 10.0 10.0 10.0)))
  (`NiagaraComponent.SetVariableLinearColor` _righteye "EyesColor" _color_2)
  (`NiagaraComponent.SetVariableLinearColor` _righteye "SparksColor" (* _color_2 (`KismetMathLibrary.MakeColor` 10.0 10.0 10.0)))
  (`SceneComponent.K2_AttachToComponent` (`self.DustRightHand`) (`self.Mesh`) "Wolf_-R-Finger0" "SnapToTarget" "SnapToTarget" "SnapToTarget" false)
  (`SceneComponent.K2_AttachToComponent` (`self.DustLeftHand`) (`self.Mesh`) "Wolf_-L-Finger0" "SnapToTarget" "SnapToTarget" "SnapToTarget" false)
  (`SceneComponent.K2_AttachToComponent` (`self.DustRightLeg`) (`self.Mesh`) "Wolf_-R-Foot" "SnapToTarget" "KeepRelative" "SnapToTarget" false)
  (`SceneComponent.K2_AttachToComponent` (`self.DustLeftLeg`) (`self.Mesh`) "Wolf_-L-Foot" "SnapToTarget" "KeepRelative" "SnapToTarget" false))