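; Numbered pressure button that calls SpawnAPawn on its CorrespondingDen when a ThirdPersonCharacter overlaps its InteractiveSpace.
; Overlap start swaps in a dimmed-color material, rescales the button on Y and plays a click; overlap end restores color and scale with another sound.
; The construction script shows ButtonNumber as text and applies ButtonColor for numbers 1 to 3.
; ChangeColor creates a new dynamic material instance on every call.
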(event `self.InteractiveSpace.OnComponentBeginOverlap`
  (params (OverlappedComponent :type "PrimitiveComponent Object Reference") (OtherActor :type "Actor Object Reference") (OtherComp :type "PrimitiveComponent Object Reference") (OtherBodyIndex :type Integer) (bFromSweep :type Boolean) (SweepResult :type "HitResult Structure (by ref)"))
  (cast `/Game/ThirdPersonBP/Blueprints/ThirdPersonCharacter` OtherActor)
  (`/Game/Blueprints/Den_BP.SpawnAPawn` (`self.CorrespondingDen`))
  (`self.Interact`))

(event `self.InteractiveSpace.OnComponentEndOverlap`
  (params (OverlappedComponent :type "PrimitiveComponent Object Reference") (OtherActor :type "Actor Object Reference") (OtherComp :type "PrimitiveComponent Object Reference") (OtherBodyIndex :type Integer))
  (cast `/Game/ThirdPersonBP/Blueprints/ThirdPersonCharacter` OtherActor)
  (`self.EndInteract`))

(event `self.Interact`
  (bind _button (`self.Button`))
  (`self.ChangeColor` (/ (`self.ButtonColor`) (`KismetMathLibrary.MakeColor` 10.0 10.0 10.0)) "/AnimationSharing/AnimSharingBlue.AnimSharingBlue" "Param")
  (`SceneComponent.SetWorldScale3D` _button (`KismetMathLibrary.MakeVector` (.x (`SceneComponent.K2_GetComponentScale` _button)) (* (.y (`SceneComponent.K2_GetComponentScale` _button)) (`self.Scale`)) (.z (`SceneComponent.K2_GetComponentScale` _button))))
  (`GameplayStatics.PlaySoundAtLocation` "/Game/SoundEffects/Click.Click" (`self.K2_GetActorLocation`) (struct) 1.0 1.0 0.0 null null null))

(event `self.EndInteract`
  (bind _button (`self.Button`))
  (`self.ChangeColor` (`self.ButtonColor`) "/Game/Materials/LaserPointerMaterialInst.LaserPointerMaterialInst" "LaserColor")
  (`SceneComponent.SetWorldScale3D` _button (`KismetMathLibrary.MakeVector` (.x (`SceneComponent.K2_GetComponentScale` _button)) (* (.y (`SceneComponent.K2_GetComponentScale` _button)) (/ 1.0 (`self.Scale`))) (.z (`SceneComponent.K2_GetComponentScale` _button))))
  (`GameplayStatics.PlaySoundAtLocation` "/Engine/EditorSounds/Notifications/CompileSuccess.CompileSuccess" (`self.K2_GetActorLocation`) (struct) 1.0 1.0 0.0 null null null))

(fn `ChangeColor`
  (params (Color :type "LinearColor Structure") (Material :type "MaterialInterface Object Reference") (ColorParamName :type Name))
  (bind _returnvalue (`KismetMaterialLibrary.CreateDynamicMaterialInstance` Material))
  (`MaterialInstanceDynamic.SetVectorParameterValue` _returnvalue ColorParamName Color)
  (`PrimitiveComponent.SetMaterial` (`self.Button`) 0 _returnvalue))

(fn `UserConstructionScript`
  (locals (Material :type "MaterialInstanceDynamic Object Reference"))
  (bind _buttoncolor (`self.ButtonColor`))
  (`TextRenderComponent.K2_SetText` (`self.TextRender`) (`KismetTextLibrary.Conv_IntToText` (`self.ButtonNumber`)))
  (switch `int` (`self.ButtonNumber`)
    (:`1`
      (bind _returnvalue (`KismetMaterialLibrary.CreateDynamicMaterialInstance` "/Game/Materials/LaserPointerMaterialInst.LaserPointerMaterialInst"))
      (bind _output_get (set `local.Material` _returnvalue))
      (`MaterialInstanceDynamic.SetVectorParameterValue` _output_get "LaserColor" _buttoncolor))
    (:`2`
      (bind _returnvalue_2 (`KismetMaterialLibrary.CreateDynamicMaterialInstance` "/Game/Materials/LaserPointerMaterialInst.LaserPointerMaterialInst"))
      (bind _output_get_2 (set `local.Material` _returnvalue_2))
      (`MaterialInstanceDynamic.SetVectorParameterValue` _output_get_2 "LaserColor" _buttoncolor))
    (:`3`
      (bind _returnvalue_3 (`KismetMaterialLibrary.CreateDynamicMaterialInstance` "/Game/Materials/LaserPointerMaterialInst.LaserPointerMaterialInst"))
      (bind _output_get_3 (set `local.Material` _returnvalue_3))
      (`MaterialInstanceDynamic.SetVectorParameterValue` _output_get_3 "LaserColor" _buttoncolor)))
  (`PrimitiveComponent.SetMaterial` (`self.Button`) 0 (`local.Material`)))