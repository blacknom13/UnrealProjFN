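; AI controller that runs the Wolf_BT behavior tree on an AIChar pawn and handles its arrival at a UFO, statue or portal.
; On begin play it caches references to those three targets.
; DestinationReached branches on PawnType to notify or interact with the matching target, starting a timer for the UFO and spawning evaporation for the statue.
; Other events halt movement through a Blackboard flag or destroy pawn and controller.
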(event `self.ReceiveBeginPlay`
  (`self.RunBehaviorTree` "/Game/AI/Wolf_BT.Wolf_BT")
  (`|ExecutionSequence`
    (:`then_0`
      (bind _outactors (`GameplayStatics.GetAllActorsOfClass` "/Game/Blueprints/UFO.UFO_C"))
      (for _array_element _outactors
        (set `self.UFORef` _array_element)))
    (:`then_1`
      (bind _outactors_2 (`GameplayStatics.GetAllActorsOfClass` "/Game/Blueprints/Portal.Portal_C"))
      (for _array_element_2 _outactors_2
        (set `self.PotalRef` _array_element_2)))
    (:`then_2`
      (bind _outactors_3 (`GameplayStatics.GetAllActorsOfClass` "/Game/Blueprints/BP_Statue.BP_Statue_C"))
      (for _array_element_3 _outactors_3
        (set `self.StatueRef` _array_element_3)))))

(event `HaltMovement`
  (`BlackboardComponent.SetValueAsBool` (`self.Blackboard`) "Stop" true))

(event `/Game/Blueprints/General_BPI.DestinationReached`
  (params (AIChar :type "/Game/Blueprints/AIChar Object Reference"))
  (bind _asaichar (cast `/Game/Blueprints/AIChar` (`self.K2_GetPawn` self)))
  (`/Game/Blueprints/General_BPI.DestinationReached` _asaichar null)
  (switch `int` (`self.PawnType`)
    (:`1`
      (`/Game/Blueprints/General_BPI.DestinationReached` (`self.UFORef`) _asaichar)
      (bind _returnvalue (`KismetSystemLibrary.K2_SetTimerDelegate` (`|CreateDelegate` :!event `DestroyActors`) 2.0))
      (set `self.TimerHandles` _returnvalue))
    (:`2`
      (`/Game/Blueprints/AIChar.SpawnEvaporation` _asaichar)
      (`/Game/Blueprints/BP_Statue.Interact` (`self.StatueRef`)))
    (:`3`
      (`/Game/Blueprints/Portal.DestinationReached` (`self.PotalRef`) _asaichar))))

(event `/Game/Blueprints/General_BPI.EndInteract`
  (`self.DestroyActors`))

(event `DestroyActors`
  (`self.K2_DestroyActor` (`self.K2_GetPawn` self))
  (`KismetSystemLibrary.K2_ClearAndInvalidateTimerHandle` (`self.TimerHandles`))
  (`self.K2_DestroyActor`))

(event `EvaporateFinished`
  (`/Game/Blueprints/BP_Statue.EndInteract` (`self.StatueRef`))
  (`self.DestroyActors`))

(fn `UserConstructionScript`)