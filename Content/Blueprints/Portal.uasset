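; Portal actor that reacts when an AI character reaches it as a destination.
; DestinationReached clears the character's end-point flag, feeds its location to the FXPortalForce effect as User.WolfLocation and activates that effect.
; It then stores the character, starts a one-shot timer whose callback is not defined here, and assigns itself to the character as its portal.
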(event `/Game/Blueprints/General_BPI.DestinationReached`
  (params (AIChar :type "/Game/Blueprints/AIChar Object Reference"))
  (bind _fx_portalforce (`self.FX_PortalForce`))
  (set `/Game/Blueprints/AIChar.ReachedEndPoint` false AIChar)
  (`NiagaraComponent.SetVariableVec3` _fx_portalforce "User.WolfLocation" (`self.K2_GetActorLocation` AIChar))
  (`ActorComponent.SetActive` _fx_portalforce true false)
  (set `self.AIChar` AIChar)
  (`KismetSystemLibrary.K2_SetTimerDelegate` (`|CreateDelegate` AIChar :!event `PortWolf`) 2.0)
  (`/Game/Blueprints/AIChar.AssignPortal` (`self.AIChar`) self))

(fn `UserConstructionScript`)